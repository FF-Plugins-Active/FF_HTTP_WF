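; Template Blueprint that runs an HTTP server actor (HTTP_Server_WF) for handling web requests on the /dyn URI.
; BeginPlay spawns the LibWebSocket-named server and binds its HTTP request delegate.
; Each request goes to a parse function that prints the URI and body on screen, then replies with a fixed test string and a custom header.
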(event Custom|DelegateHttpRequest_Event
  (params (Request :type Http%20Request%20Wf%20Object%20Reference))
  (CallFunction|FParseRequest Request))

(event EventBeginPlay
  (bind _returnvalue (Game|SpawnActorfromClass "/Script/FF_HTTP_WF.HTTP_Server_WF" (Math|Transform|MakeTransform "0, 0, 0" "0, 0, 0" "1.000000,1.000000,1.000000") "Undefined" "MultiplyWithRoot" 0 "/dyn" "LibWebSocket" 8081 8453 4 0))
  (bind _output_get (Variables|Default|SetServer_WF _returnvalue))
  (EventDispatchers|AssignDelegateHttpRequest _output_get (delegate Custom|DelegateHttpRequest_Event)))

(fn ConstructionScript)

(fn FParseRequest
  (params (In_Request :type Http%20Request%20Wf%20Object%20Reference))
  (LocalVariables|SetLOC_Request In_Request)
  (bind _out_uri (Class|HttpRequestWf|GetRequestUri (LocalVariables|GetLOC_Request)))
  (Development|PrintString _out_uri true true "(R=0.000000,G=0.660000,B=1.000000,A=1.000000)" 3e+01)
  (bind _out_body (Class|HttpRequestWf|GetBody (LocalVariables|GetLOC_Request)))
  (Development|PrintString _out_body true true "(R=0.000000,G=0.660000,B=1.000000,A=1.000000)" 3e+01)
  (Class|HttpRequestWf|SendResponseString (LocalVariables|GetLOC_Request) (Utilities|Map|MakeMap "frozen forest" "digital twin") "test" "OK_200" "Text_Plain")
  (return))